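; BonFire_BP is a bonfire that saves the world when interacted with.
; Interact sets FireActivate, calls WriteSaveGame on BuptGameModeBase, prints a confirmation and runs UpdateFlames, which activates the particle system if the flag is set.
; OnActorLoaded also runs UpdateFlames, so the flame effect follows the flag when the actor loads.
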(event `UpdateFlames`
  (if (`self.bFireActivate`)
    (`ActorComponent.Activate` (`self.ParticleSystem`) false)))

(event `BuptGamePlayInterface.Interact`
  (params (InstigatorPawn :type "Pawn Object Reference"))
  (set `self.bFireActivate` true)
  (bind _asbupt_game_mode_base (cast `BuptGameModeBase` (`GameplayStatics.GetGameMode`)))
  (`BuptGameModeBase.WriteSaveGame` _asbupt_game_mode_base)
  (`KismetSystemLibrary.PrintString` "WORLD SAVED!")
  (`self.UpdateFlames`))

(event `BuptGamePlayInterface.OnActorLoaded`
  (`self.UpdateFlames`))

(fn `UserConstructionScript`)