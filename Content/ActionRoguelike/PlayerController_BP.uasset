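; Local player controller for an action roguelike that sets up the player's HUD and offers a manual save shortcut.
; When play begins for a local controller, it creates the Main_HUD widget, adds it to the viewport and switches input to game-only.
; Pressing L casts the game mode to BuptGameModeBase, calls its save-game write and prints a confirmation message.
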(event `self.ReceiveBeginPlay`)

(event `self.BlueprintBeginPlayingState`
  (if (`self.IsLocalController`)
    (bind _returnvalue (`|CreateWidget` "/Game/ActionRoguelike/UI/Main_HUD.Main_HUD_C"))
    (`UserWidget.AddToViewport` _returnvalue 0)
    (`WidgetBlueprintLibrary.SetInputMode_GameOnly` self)))

(event `Key|L`
  (params (Key :type "Key Structure"))
  (:`Pressed`
    (bind _asbupt_game_mode_base (cast `BuptGameModeBase` (`GameplayStatics.GetGameMode`)))
    (`BuptGameModeBase.WriteSaveGame` _asbupt_game_mode_base)
    (`KismetSystemLibrary.PrintString` "WORLD SAVED!")))

(fn `UserConstructionScript`)